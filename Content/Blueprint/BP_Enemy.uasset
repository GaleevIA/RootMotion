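; Enemy Blueprint that alternates between charging the third-person player and retreating to a random offset point, flipping on arrival.
; Each Tick, a visibility trace picks the direct destination or, when blocked, CheckPath takes the next navmesh path point.
; It updates Speed by distance and Turn toward that point, but applies no movement itself.
; While retreating or near its destination, it smoothly rotates to face the player.
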(event EventBeginPlay
  (bind _returnvalue (Actor|GetActorOfClass "/Game/ThirdPerson/Blueprints/BP_ThirdPersonCharacter.BP_ThirdPersonCharacter_C"))
  (Variables|Default|SetPlayer _returnvalue)
  (Variables|Default|SetDirection 1.0)
  (Variables|Default|SetSpeed 1.0))

(event EventTick
  (params (DeltaSeconds :type Float%20%28single-precision%29))
  (bind _player (Variables|Default|GetPlayer))
  (bind _returnvalue (Transformation|GetActorLocation _player))
  ;[1 1 1] Если точка назначения это персонаж, то обновляем ее при изменении позиции игрока
  (if (== (Variables|Default|GetDirection) 1.0)
    (Variables|Default|SetDestination _returnvalue))
  ;[1 1 1] Если персонаж не может дойти до игрока напрямую, то выбирается ближайшая точка обхода
  (bind _outhit (Collision|LineTraceByChannel (Transformation|GetActorLocation) (Variables|Default|GetDestination) "TraceTypeQuery1" false 0 "None"))
  (if (.bBlockingHit (Collision|BreakHitResult _outhit))
    (CallFunction|CheckPath)
    (else
      (Variables|Default|SetCurDestination (Variables|Default|GetDestination))))
  ;[1 1 1] Обновляем угол поворота персонажа
  (CallFunction|ChangeTurnAngle _returnvalue DeltaSeconds)
  ;[1 1 1] Если персонаж приблизился к точке назначения, меняем направление движения и генерируем новую точку назначения
  (if (< (Math|Vector|VectorLength (- (Transformation|GetActorLocation) (Variables|Default|GetDestination))) 4e+02)
    (Variables|Default|SetSpeed 1.5))
  (if (< (Math|Vector|VectorLength (- (Transformation|GetActorLocation) (Variables|Default|GetDestination))) 2.5e+02)
    (Variables|Default|SetSpeed 2.0))
  (if (< (Math|Vector|VectorLength (- (Transformation|GetActorLocation) (Variables|Default|GetDestination))) 1.3e+02)
    (CallFunction|ChangeDirection)
    (if (== (Variables|Default|GetDirection) -1.0)
      (CallFunction|ChangeDestination))
    (Variables|Default|SetSpeed 1.0)))

(fn ConstructionScript)

(fn ChangeDirection
  ;[1 1 1] 1 - персонаж бежит на игрока, -1 - персонаж бежит от игрока
  (Variables|Default|SetDirection (* (Variables|Default|GetDirection) -1.0)))

(fn ChangeDestination
  (bind _returnvalue (Transformation|GetActorLocation))
  ;[1 1 1] Выбираем новую точку назначения исходя из заданных значений радиуса
  (bind _output_get (Variables|Default|SetDestination (Math|Vector|MakeVector (+ (Math|Random|RandomFloatinRange (Variables|Default|GetMinDestinationRadius) (Variables|Default|GetMaxDestinationRadius)) (.x _returnvalue)) (+ (Math|Random|RandomFloatinRange (Variables|Default|GetMinDestinationRadius) (Variables|Default|GetMaxDestinationRadius)) (.y _returnvalue)) 5e+01)))
  (Rendering|Debug|DrawDebugBox _output_get "10.000000,10.000000,100.000000" "(R=0.781250,G=0.087708,B=0.000000,A=1.000000)" "0, 0, 0" 1e+01 0.0))

(fn ChangeTurnAngle
  (params (PlayerLocation :type Vector) (DeltaTime :type Float%20%28double-precision%29))
  (Variables|Default|SetTurn (.yaw (Math|Rotator|Delta(Rotator) (Math|Rotator|FindLookatRotation (Transformation|GetActorLocation) (Variables|Default|GetCurDestination)) (Transformation|GetActorRotation))))
  (if (or (== (Variables|Default|GetDirection) -1.0) (< (Math|Vector|VectorLength (- (Transformation|GetActorLocation) (Variables|Default|GetDestination))) 4e+02))
    (Transformation|SetActorRotation (Math|Interpolation|RInterpTo (Transformation|GetActorRotation) (Math|Rotator|FindLookatRotation (Transformation|GetActorLocation) PlayerLocation) DeltaTime 5.0))))

(fn CheckPath
  (bind _returnvalue (Class|NavigationSystemV1|FindPathtoLocationSynchronously (Transformation|GetActorLocation) (Variables|Default|GetDestination) 0 "/Script/AIModule.NavFilter_AIControllerDefault"))
  (bind _output_get (Variables|Default|SetPath%20Points (Variables|/Script/NavigationSystem.NavigationPath|GetPathPoints _returnvalue)))
  (bind _output_get_2 (Variables|Default|SetCurDestination (Utilities|Array|Get(acopy) _output_get 1)))
  (Rendering|Debug|DrawDebugBox _output_get_2 "10.000000,10.000000,100.000000" "(R=0.541667,G=0.000000,B=0.036884,A=1.000000)" "0, 0, 0" 1.0 0.0))